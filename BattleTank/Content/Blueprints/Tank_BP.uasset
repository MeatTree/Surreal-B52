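; Tank_BP is the player-controlled tank Blueprint that wires input to components and passes its barrel and turret references on at BeginPlay.
; Aim axes rotate an azimuth gimbal in yaw and the spring arm in pitch.
; Separate left and right throttle axes drive each track component independently, and the Fire action calls Fire.
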(event EventBeginPlay
  (Class|Tank|SetBarrelReference (Variables|Default|GetTankBarrel))
  (Class|Tank|SetTurretReference (Variables|Default|GetTankTurret)))

(event Input|ActionEvents|InputActionFire
  (params (Key :type Key%20Structure))
  ;[1 1 1] Aim Input Bindings
  (:Pressed
    (Class|Tank|Fire)))

(event Input|AxisEvents|InputAxisAimAzimuth
  (params (AxisValue :type Float%20%28single-precision%29))
  ;[1 1 1] Aim Input Bindings
  (Transformation|AddLocalRotation (Variables|Default|GetAzimoth%20Gimbal) (Math|Rotator|MakeRotator 0.0 0.0 AxisValue) false false))

(event Input|AxisEvents|InputAxisLeftTrackThrottle
  (params (AxisValue :type Float%20%28single-precision%29))
  ;[1 1 1] Throttle Input Bindings
  (Class|TankTrack|SetThrottle (Variables|Default|GetTankTrackLeft) AxisValue))

(event Input|AxisEvents|InputAxisRightTrackThrottle
  (params (AxisValue :type Float%20%28single-precision%29))
  ;[1 1 1] Throttle Input Bindings
  (Class|TankTrack|SetThrottle (Variables|Default|GetTankTrackRight) AxisValue))

(event Input|AxisEvents|InputAxisAimElevation
  (params (AxisValue :type Float%20%28single-precision%29))
  ;[1 1 1] Aim Input Bindings
  (Transformation|AddLocalRotation (Variables|Default|GetSpringArm) (Math|Rotator|MakeRotator 0.0 AxisValue 0.0) false false))

(fn ConstructionScript)